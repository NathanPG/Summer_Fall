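; Game State for a timed brawl that counts down the match, tracks the high score and collapses the arena.
; Tick sends time and high score to players, while the authority drops actors tagged first, second and third by enabling physics, randomly then all at once, with warnings per level.
; At zero, it names a best player having both the top score and the fewest deaths overall, then ends and pauses the game.
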(event `GetBestPlayer`
  (bind _output (`|GetArrayItem` (`self.BestPlayersWithMinDeath`)))
  (for _array_element (`self.PlayerArray`)
    (bind _asbp_player_state (cast `/Game/Blueprints/Player/BP_PlayerState` _array_element))
    (bind _deathcount (`/Game/Blueprints/Player/BP_PlayerState.DeathCount` _asbp_player_state))
    (if (<= _deathcount (`self.MinDeath`))
      (set `self.MinDeath` _deathcount)))
  (for _array_element_2 (`self.PlayerArray`)
    (bind _asbp_player_state_2 (cast `/Game/Blueprints/Player/BP_PlayerState` _array_element_2))
    (if (== (`/Game/Blueprints/Player/BP_PlayerState.DeathCount` _asbp_player_state_2) (`self.MinDeath`))
      (if (== (`/Game/Blueprints/Player/BP_PlayerState.PlayerScore` _asbp_player_state_2) (`self.HighestScore`))
        (`KismetArrayLibrary.Array_Add` (`self.BestPlayersWithMinDeath`) _asbp_player_state_2))))
  (`/Engine/EditorBlueprintResources/StandardMacros.IsValid` _output
    (:`Is Valid`
      (set `self.BestPlayer` (`KismetTextLibrary.Conv_StringToText` (`PlayerState.PlayerName` _output))))))

(event `self.ReceiveTick`
  (params (DeltaSeconds :type "Float (single-precision)"))
  (bind _first (`self.First`))
  (bind _second (`self.Second`))
  (bind _third (`self.Third`))
  (bind _output (`|GetArrayItem` _third (`KismetMathLibrary.RandomIntegerInRange` 0 (`KismetArrayLibrary.Array_Length` _third))))
  (bind _output_2 (`|GetArrayItem` _first (`KismetMathLibrary.RandomIntegerInRange` 0 (`KismetArrayLibrary.Array_Length` _first))))
  (bind _output_3 (`|GetArrayItem` _second (`KismetMathLibrary.RandomIntegerInRange` 0 (`KismetArrayLibrary.Array_Length` _second))))
  (set `self.Time` (- (`self.Time`) DeltaSeconds))
  (`|ExecutionSequence`
    (:`then_0`
      (bind _outactors (`GameplayStatics.GetAllActorsOfClass` "/Game/Blueprints/Player/Player_Base.Player_Base_C"))
      (for _array_element _outactors
        (`/Game/Blueprints/Player/Player_Base.Time_Multi` _array_element (`self.Time`))))
    (:`then_1`
      (`KismetSystemLibrary.Delay` 1.0)
      (for _array_element_2 (`self.PlayerArray`)
        (bind _asbp_player_state (cast `/Game/Blueprints/Player/BP_PlayerState` _array_element_2))
        (bind _playerscore (`/Game/Blueprints/Player/BP_PlayerState.PlayerScore` _asbp_player_state))
        (`/Engine/EditorBlueprintResources/StandardMacros.CompareInt` _playerscore (`self.HighestScore`)
          (:`>`
            (bind _output_get (set `self.HighestScore` _playerscore))
            (for _array_element_3 (`self.PlayerArray`)
              (bind _asbp_player_state_2 (cast `/Game/Blueprints/Player/BP_PlayerState` _array_element_3))
              (`/Game/Blueprints/Player/BP_PlayerState.Highest_Multi` _asbp_player_state_2 _output_get))))))
    (:`then_2`
      (`/Engine/EditorBlueprintResources/ActorMacros.Switch Has Authority`
        (:`Authority`
          (`|ExecutionSequence`
            (:`then_0`
              (if (not (`self.FirstFallen`))
                (`KismetSystemLibrary.Delay` 0.3)
                (if (<= (`KismetMathLibrary.FTrunc` (`self.Time`)) 175)
                  (`/Engine/EditorBlueprintResources/StandardMacros.IsValid` _output_2
                    (:`Is Valid`
                      (bind _asstatic_mesh_actor (cast `StaticMeshActor` _output_2))
                      (`self.SetSP_Multi` (`StaticMeshActor.StaticMeshComponent` _asstatic_mesh_actor))
                      (`/Engine/EditorBlueprintResources/StandardMacros.DoOnce` false
                        (:`Completed`
                          (`GameplayStatics.PlaySound2D` "/Game/Audio/Warning_Cue.Warning_Cue" 1.0 1.0 0.0 null null)
                          (bind _outactors_2 (`GameplayStatics.GetAllActorsOfClass` "/Game/Blueprints/Player/Player_Base.Player_Base_C"))
                          (for _array_element_4 _outactors_2
                            (bind _ui (`/Game/Blueprints/Player/Player_Base.UI` _array_element_4))
                            (`/Engine/EditorBlueprintResources/StandardMacros.IsValid` _ui
                              (:`Is Valid`
                                (`/Game/Blueprints/UI/GameUI.ShowWarning` _ui "Warning! The Bottom Level Is Falling!")))))))))))
            (:`then_1`
              (if (== (`KismetMathLibrary.FTrunc` (`self.Time`)) 100)
                (set `self.FirstFallen` true)
                (for _array_element_5 (`self.First`)
                  (`/Engine/EditorBlueprintResources/StandardMacros.IsValid` _array_element_5
                    (:`Is Valid`
                      (bind _asstatic_mesh_actor_2 (cast `StaticMeshActor` _array_element_5)
                        (:`then`
                          (`self.SetSP_Multi` (`StaticMeshActor.StaticMeshComponent` _asstatic_mesh_actor_2)))
                        (:`CastFailed`
                          (`self.Destroy_Multi` _array_element_5))))))))
            (:`then_2`
              (if (not (`self.SecondFallen`))
                (`KismetSystemLibrary.Delay` 0.4)
                (if (<= (`KismetMathLibrary.FTrunc` (`self.Time`)) 90)
                  (`/Engine/EditorBlueprintResources/StandardMacros.IsValid` _output_3
                    (:`Is Valid`
                      (bind _asstatic_mesh_actor_3 (cast `StaticMeshActor` _output_3))
                      (`self.SetSP_Multi` (`StaticMeshActor.StaticMeshComponent` _asstatic_mesh_actor_3))
                      (`/Engine/EditorBlueprintResources/StandardMacros.DoOnce` false
                        (:`Completed`
                          (bind _outactors_3 (`GameplayStatics.GetAllActorsOfClass` "/Game/Blueprints/Player/Player_Base.Player_Base_C"))
                          (for _array_element_6 _outactors_3
                            (`/Game/Blueprints/UI/GameUI.ShowWarning` (`/Game/Blueprints/Player/Player_Base.UI` _array_element_6) "Warning! The Middle Level Is Falling!")))))))))
            (:`then_3`
              (if (== (`KismetMathLibrary.FTrunc` (`self.Time`)) 60)
                (set `self.SecondFallen` true)
                (for _array_element_7 (`self.Second`)
                  (`/Engine/EditorBlueprintResources/StandardMacros.IsValid` _array_element_7
                    (:`Is Valid`
                      (bind _asstatic_mesh_actor_4 (cast `StaticMeshActor` _array_element_7)
                        (:`then`
                          (`self.SetSP_Multi` (`StaticMeshActor.StaticMeshComponent` _asstatic_mesh_actor_4)))
                        (:`CastFailed`
                          (`self.Destroy_Multi` _array_element_7))))))))
            (:`then_4`
              (if (not (`self.ThirdFallen`))
                (`KismetSystemLibrary.Delay` 0.5)
                (if (<= (`KismetMathLibrary.FTrunc` (`self.Time`)) 30)
                  (`/Engine/EditorBlueprintResources/StandardMacros.IsValid` _output
                    (:`Is Valid`
                      (bind _asstatic_mesh_actor_5 (cast `StaticMeshActor` _output))
                      (`self.SetSP_Multi` (`StaticMeshActor.StaticMeshComponent` _asstatic_mesh_actor_5))
                      (`/Engine/EditorBlueprintResources/StandardMacros.DoOnce` false
                        (:`Completed`
                          (bind _outactors_4 (`GameplayStatics.GetAllActorsOfClass` "/Game/Blueprints/Player/Player_Base.Player_Base_C"))
                          (for _array_element_8 _outactors_4
                            (`/Game/Blueprints/UI/GameUI.ShowWarning` (`/Game/Blueprints/Player/Player_Base.UI` _array_element_8) "Warning! The Top Level Is Falling!")))))))))
            (:`then_5`
              (if (== (`KismetMathLibrary.FTrunc` (`self.Time`)) 0)
                (set `self.ThirdFallen` true)
                (for _array_element_9 (`self.Third`)
                  (`/Engine/EditorBlueprintResources/StandardMacros.IsValid` _array_element_9
                    (:`Is Valid`
                      (bind _asstatic_mesh_actor_6 (cast `StaticMeshActor` _array_element_9)
                        (:`then`
                          (`self.SetSP_Multi` (`StaticMeshActor.StaticMeshComponent` _asstatic_mesh_actor_6)))
                        (:`CastFailed`
                          (`self.Destroy_Multi` _array_element_9))))))))))))
    (:`then_3`
      (if (<= (`self.Time`) 0.0)
        (`/Engine/EditorBlueprintResources/StandardMacros.DoOnce` false
          (:`Completed`
            (`self.GetBestPlayer`)
            (bind _outactors_5 (`GameplayStatics.GetAllActorsOfClass` "/Game/Blueprints/Player/Player_Base.Player_Base_C"))
            (for _array_element_10 _outactors_5
              (`/Game/Blueprints/Player/Player_Base.GameEnd` _array_element_10)
              (`GameplayStatics.SetGamePaused` true))))))))

(event `self.ReceiveBeginPlay`
  (bind _outactors (`GameplayStatics.GetAllActorsWithTag` "first"))
  (set `self.First` _outactors)
  (bind _outactors_2 (`GameplayStatics.GetAllActorsWithTag` "second"))
  (set `self.Second` _outactors_2)
  (bind _outactors_3 (`GameplayStatics.GetAllActorsWithTag` "third"))
  (set `self.Third` _outactors_3)
  (`GameplayStatics.SetGamePaused` false))

(event `SetSP_Multi`
  (params (targetOBJ :type "PrimitiveComponent Object Reference"))
  (`PrimitiveComponent.SetSimulatePhysics` targetOBJ true))

(event `Destroy_Multi`
  (params (targetOBJ :type "Actor Object Reference"))
  (`self.K2_DestroyActor` targetOBJ))

(fn `OnRep_Name`)

(fn `OnRep_NameArray`)

(fn `OnRep_NameTaken`)

(fn `OnRep_UsedIndex`)

(fn `UserConstructionScript`)