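; Base player character for a multiplayer pushing game, handling movement, dashing, pushing players and crates, timed speed/strength buffs, freeze, respawn and game-over view.
; Push combines a crate line trace with cone-overlap player tracking, while dash hits launch players or crates.
; Actions branch on authority into server or multicast events, though some server launches apply directly.
; Pushes record the attacker's PlayerId temporarily, and BeKilled_Multi awards score to a given killer ID.
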(event `Key|Tab`
  (params (Key :type "Key Structure"))
  (:`Pressed`
    (`/Engine/EditorBlueprintResources/StandardMacros.DoOnce` false :!label _label
      (:`Completed`
        (bind _returnvalue (`|CreateWidget` "/Game/Blueprints/UI/PlayerList.PlayerList_C" (`GameplayStatics.GetPlayerController` 0)))
        (bind _output_get (set `self.List` _returnvalue))
        (`UserWidget.AddToViewport` _output_get 0)
        (`KismetSystemLibrary.RetriggerableDelay` 2.0)
        (`Widget.SetVisibility` (`self.List`) "Hidden")
        (goto _label :!via `Reset`)))))

(event `CastBuff_Server`
  (params (type :type Integer))
  (`self.CastBuff_Multi` type))

(event `Key|Z`
  (params (Key :type "Key Structure"))
  (bind _bufftype (`self.BuffType`))
  (:`Pressed`
    (if (not (== (`self.BuffType`) -1))
      (`/Game/Blueprints/UI/GameUI.UsedBuff` (`self.UI`))
      (`/Engine/EditorBlueprintResources/ActorMacros.Switch Has Authority`
        (:`Authority`
          (`self.CastBuff_Multi` _bufftype))
        (:`Remote`
          (`self.CastBuff_Server` _bufftype))))))

(event `CastBuff_Multi`
  (params (type :type Integer))
  (bind _bufftime (`self.BuffTime`))
  (switch `int` type
    (:`0`
      (`self.SpeedPowerUp_Multi` _bufftime)
      (set `self.BuffType` -1))
    (:`1`
      (`self.StrengthPowerUp_Multi` _bufftime))))

(event `GetBuff`
  (params (type :type Integer))
  (bind _ui (`self.UI`))
  (bind _output_get (set `self.BuffType` type))
  (`/Engine/EditorBlueprintResources/StandardMacros.IsValid` _ui
    (:`Is Valid`
      (`/Game/Blueprints/UI/GameUI.BuffUI` _ui _output_get))))

(event `StrengthPowerUp_Multi`
  (params (EffectTIme :type "Float (double-precision)"))
  (set `self.PushPlayerForce` 600.0)
  (set `self.PushCrateForce` 600.0)
  (`KismetSystemLibrary.RetriggerableDelay` EffectTIme)
  (set `self.PushPlayerForce` 400.0)
  (set `self.PushCrateForce` 500.0))

(event `Destroy_Server`
  (params (target :type "Actor Object Reference"))
  (`self.Destroy_Multi` target))

(event `SpeedPowerUp_Multi`
  (params (EffectTime :type "Float (double-precision)"))
  (bind _charactermovement (`self.CharacterMovement`))
  (set `CharacterMovementComponent.MaxWalkSpeed` 500.0 _charactermovement)
  (`KismetSystemLibrary.RetriggerableDelay` EffectTime)
  (set `CharacterMovementComponent.MaxWalkSpeed` 250.0 _charactermovement))

(event `Destroy_Multi`
  (params (target :type "Actor Object Reference"))
  (`self.K2_DestroyActor` target))

(event `self.ReceiveTick`
  (params (DeltaSeconds :type "Float (single-precision)"))
  (`|ExecutionSequence`
    (:`then_0`
      (if (`self.DashCharging`)
        (bind _output_get (set `self.DashCoolDown` (- (`self.DashCoolDown`) DeltaSeconds)))
        (if (<= _output_get 0.0)
          (set `self.DashCharging` false)
          (set `self.DashCoolDown` 3.0))))))

(event `self.ReceiveBeginPlay`
  (set `self.SpawnLocation` (`SceneComponent.K2_GetComponentLocation` (`self.CapsuleComponent`)))
  (if (not (`self.IsLocallyControlled`))
    (`SceneComponent.SetHiddenInGame` (`self.Widget`) false false)))

(event `Launch_Server`
  (params (Target :type "PlayerCharacter Object Reference (by ref)") (LaunchVelocity :type "Vector Structure"))
  (`self.LaunchCharacter` Target LaunchVelocity false false))

(event `Launch_Multi`
  (params (Target :type "PlayerCharacter Object Reference (by ref)") (LaunchVelocity :type "Vector Structure"))
  (`self.LaunchCharacter` Target LaunchVelocity false false))

(event `PushCrate_Multi`
  (params (Target :type "PrimitiveComponent Object Reference (by ref)") (LaunchVelocity :type "Vector Structure"))
  (`PrimitiveComponent.AddImpulse` Target LaunchVelocity "None" true))

(event `PushCrate_Server`
  (params (Target :type "PrimitiveComponent Object Reference (by ref)") (LaunchVelocity :type "Vector Structure"))
  (`self.PushCrate_Multi` Target LaunchVelocity))

(event `InputAction|Push`
  (params (Key :type "Key Structure"))
  (bind _contactedplayers (`self.ContactedPlayers`))
  (bind _returnvalue (`SceneComponent.K2_GetComponentLocation` (`self.CapsuleComponent`)))
  (bind _playerid (`PlayerState.PlayerId` (`self.PlayerState`)))
  (bind _returnvalue_2 (`KismetMathLibrary.MakeVector` (.x (* (`KismetMathLibrary.Normal` (`self.GetActorForwardVector`)) (`self.PushCrateForce`))) (.y (* (`KismetMathLibrary.Normal` (`self.GetActorForwardVector`)) (`self.PushCrateForce`))) 200.0))
  (:`Pressed`
    (`|ExecutionSequence`
      (:`then_0`
        (`/Engine/EditorBlueprintResources/StandardMacros.DoOnce` false :!label _label_2
          (:`Completed`
            (`/Engine/EditorBlueprintResources/ActorMacros.Switch Has Authority`
              (:`Authority`
                (`self.PushAnim_Multi`))
              (:`Remote`
                (`self.PushAnim_Server`)))
            (`|ExecutionSequence`
              (:`then_0`
                (bind (_outhit _returnvalue_3) (`KismetSystemLibrary.LineTraceSingle` _returnvalue (+ _returnvalue (* (`KismetMathLibrary.Normal` (`SceneComponent.GetForwardVector` (`self.CapsuleComponent`))) 100.0)) "TraceTypeQuery2"))
                (if _returnvalue_3
                  (bind _ascrate (cast `/Game/Blueprints/Level/Crate` (`.HitActor` (`GameplayStatics.BreakHitResult` _outhit))))
                  (`/Engine/EditorBlueprintResources/ActorMacros.Switch Has Authority`
                    (:`Authority`
                      (bind _staticmesh (`/Game/Blueprints/Level/Crate.StaticMesh` _ascrate))
                      (`self.PushCrate_Multi` _staticmesh _returnvalue_2))
                    (:`Remote`
                      (`self.PushCrate_Server` _staticmesh _returnvalue_2)))))
              (:`then_1`
                (if (not (== (`KismetArrayLibrary.Array_Length` _contactedplayers) 0))
                  (for _array_element _contactedplayers
                    (if (not (`self.IsLocallyControlled` _array_element))
                      (`/Engine/EditorBlueprintResources/ActorMacros.Switch Has Authority`
                        (:`Authority`
                          (bind _returnvalue_4 (`KismetMathLibrary.MakeVector` (.x (* (`KismetMathLibrary.Normal` (- (`SceneComponent.K2_GetComponentLocation` (`Character.CapsuleComponent` _array_element)) (`SceneComponent.K2_GetComponentLocation` (`self.CapsuleComponent`)))) (`self.PushPlayerForce`))) (.y (* (`KismetMathLibrary.Normal` (- (`SceneComponent.K2_GetComponentLocation` (`Character.CapsuleComponent` _array_element)) (`SceneComponent.K2_GetComponentLocation` (`self.CapsuleComponent`)))) (`self.PushPlayerForce`))) 200.0))
                          (`self.Launch_Multi` _array_element _returnvalue_4)
                          (`self.LastPush_Multi` _playerid _array_element))
                        (:`Remote`
                          (`self.Launch_Server` _array_element _returnvalue_4)
                          (`self.LastPush_Server` _playerid _array_element)))))))))))
      (:`then_1`
        (`KismetSystemLibrary.Delay` 1.0)
        (goto _label_2 :!via `Reset`)))))

(event `PushAnim_Server`
  (`self.PushAnim_Multi`))

(event `PushAnim_Multi`
  (`|PlayMontage` (`self.Mesh`) "/Game/ArtAssets/scifi/pushtest_Anim_Montage.pushtest_Anim_Montage" 1.5))

(event `self.Cone.OnComponentBeginOverlap`
  (params (OverlappedComponent :type "PrimitiveComponent Object Reference") (OtherActor :type "Actor Object Reference") (OtherComp :type "PrimitiveComponent Object Reference") (OtherBodyIndex :type Integer) (bFromSweep :type Boolean) (SweepResult :type "HitResult Structure (by ref)"))
  (bind _asplayer_base (cast `/Game/Blueprints/Player/Player_Base` OtherActor))
  (`KismetArrayLibrary.Array_Add` (`self.ContactedPlayers`) _asplayer_base))

(event `self.Cone.OnComponentEndOverlap`
  (params (OverlappedComponent :type "PrimitiveComponent Object Reference") (OtherActor :type "Actor Object Reference") (OtherComp :type "PrimitiveComponent Object Reference") (OtherBodyIndex :type Integer))
  (bind _asplayer_base (cast `/Game/Blueprints/Player/Player_Base` OtherActor))
  (`KismetArrayLibrary.Array_RemoveItem` (`self.ContactedPlayers`) _asplayer_base))

(event `self.ReceiveHit`
  (params (MyComp :type "PrimitiveComponent Object Reference") (Other :type "Actor Object Reference") (OtherComp :type "PrimitiveComponent Object Reference") (bSelfMoved :type Boolean) (HitLocation :type "Vector Structure") (HitNormal :type "Vector Structure") (NormalImpulse :type "Vector Structure") (Hit :type "HitResult Structure (by ref)"))
  (bind _playerid (`PlayerState.PlayerId` (`self.PlayerState`)))
  (bind _returnvalue (`KismetMathLibrary.MakeVector` (.x (* (`KismetMathLibrary.Normal` (`self.GetActorForwardVector`)) (`self.PushCrateForce`))) (.y (* (`KismetMathLibrary.Normal` (`self.GetActorForwardVector`)) (`self.PushCrateForce`))) 200.0))
  (bind _returnvalue_2 (`KismetMathLibrary.MakeVector` (.x (* (`KismetMathLibrary.Normal` (`self.GetActorForwardVector`)) (`self.DashVelocity`))) (.y (* (`KismetMathLibrary.Normal` (`self.GetActorForwardVector`)) (`self.DashVelocity`))) 100.0))
  (if (`self.Dashing`)
    (bind _asplayer_base (cast `/Game/Blueprints/Player/Player_Base` Other)
      (:`then`
        (`KismetSystemLibrary.PrintString` "Dash Hit Player!")
        (`/Engine/EditorBlueprintResources/ActorMacros.Switch Has Authority`
          (:`Authority`
            (`self.DashPush_Multi` _asplayer_base _returnvalue_2)
            (set `self.Dashing` false)
            (`self.LastPush_Multi` _asplayer_base _playerid _asplayer_base))
          (:`Remote`
            (`self.DashPush_Server` _asplayer_base _returnvalue_2)
            (set `self.Dashing` false)
            (`self.LastPush_Server` _asplayer_base _playerid _asplayer_base))))
      (:`CastFailed`
        (bind _ascrate (cast `/Game/Blueprints/Level/Crate` Other))
        (`KismetSystemLibrary.PrintString` "Crate")
        (`/Engine/EditorBlueprintResources/ActorMacros.Switch Has Authority`
          (:`Authority`
            (bind _staticmesh (`/Game/Blueprints/Level/Crate.StaticMesh` _ascrate))
            (`self.PushCrate_Multi` _staticmesh _returnvalue))
          (:`Remote`
            (`self.PushCrate_Server` _staticmesh _returnvalue)))))))

(event `DashPush_Server`
  (params (Target :type "PlayerCharacter Object Reference (by ref)") (LaunchVelocity :type "Vector Structure"))
  (`self.LaunchCharacter` Target LaunchVelocity false false)
  (`KismetSystemLibrary.Delay` 0.5)
  (set `self.Dashing` false))

(event `DashPush_Multi`
  (params (Target :type "PlayerCharacter Object Reference (by ref)") (LaunchVelocity :type "Vector Structure"))
  (`self.LaunchCharacter` Target LaunchVelocity false false)
  (`KismetSystemLibrary.Delay` 0.5)
  (set `self.Dashing` false))

(event `DashCrate_Server`
  (params (Target :type "PrimitiveComponent Object Reference (by ref)") (LaunchVelocity :type "Vector Structure"))
  (`PrimitiveComponent.AddImpulse` Target LaunchVelocity "None" true))

(event `DashCrate_Multi`
  (params (Target :type "PrimitiveComponent Object Reference (by ref)") (LaunchVelocity :type "Vector Structure"))
  (`self.PushCrate_Multi` Target LaunchVelocity))

(event `LastPush_Server`
  (params (WhoPushed :type Integer) (BePushed :type "PlayerCharacter Object Reference (by ref)"))
  (`/Engine/EditorBlueprintResources/ActorMacros.Switch Has Authority`
    (:`Authority`
      (`self.LastPush_Multi` WhoPushed BePushed))))

(event `InputAxis|MoveForward` :overrideparent false
  (params (AxisValue :type "Float (single-precision)"))
  (if (`self.Dashing`)
    _
    (elif (`self.EnableMove`)
      (`self.AddMovementInput` (`KismetMathLibrary.GetForwardVector` (`KismetMathLibrary.MakeRotator` 0.0 0.0 (.yaw (`self.GetControlRotation`)))) AxisValue))))

(event `InputAxis|MoveRight` :overrideparent false
  (params (AxisValue :type "Float (single-precision)"))
  (if (`self.Dashing`)
    _
    (elif (`self.EnableMove`)
      (`self.AddMovementInput` (`KismetMathLibrary.GetRightVector` (`KismetMathLibrary.MakeRotator` 0.0 0.0 (.yaw (`self.GetControlRotation`)))) AxisValue))))

(event `InputAxis|Turn` :overrideparent false
  (params (AxisValue :type "Float (single-precision)"))
  (`self.AddControllerYawInput` (* AxisValue 0.5)))

(event `Dash_Multi`
  (params (Target :type "PlayerCharacter Object Reference (by ref)") (LaunchVelocity :type "Vector Structure"))
  (`self.LaunchCharacter` Target LaunchVelocity true true)
  (`|PlayMontage` (`self.Mesh`) "/Game/ArtAssets/scifi/cyborgdashpose_Anim_Montage.cyborgdashpose_Anim_Montage" 2.0))

(event `Dash_Server`
  (params (Target :type "PlayerCharacter Object Reference (by ref)") (LaunchVelocity :type "Vector Structure"))
  (`self.Dash_Multi` Target LaunchVelocity))

(event `InputAction|Dash`
  (params (Key :type "Key Structure"))
  (bind _returnvalue (`KismetMathLibrary.MakeVector` (.x (* (`KismetMathLibrary.Normal` (`self.GetActorForwardVector`)) (`self.DashVelocity`))) (.y (* (`KismetMathLibrary.Normal` (`self.GetActorForwardVector`)) (`self.DashVelocity`))) 200.0))
  (:`Pressed`
    (if (not (`self.DashCharging`))
      (set `self.DashCharging` true)
      (set `self.Dashing` true)
      (`/Engine/EditorBlueprintResources/ActorMacros.Switch Has Authority`
        (:`Authority`
          (`self.Dash_Multi` self _returnvalue)
          (`KismetSystemLibrary.Delay` 0.3)
          (set `self.Dashing` false))
        (:`Remote`
          (`self.Dash_Server` self _returnvalue)
          (`KismetSystemLibrary.Delay` 0.3)
          (set `self.Dashing` false))))))

(event `LastPush_Multi`
  (params (WhoPushed :type Integer) (BePushed :type "PlayerCharacter Object Reference (by ref)"))
  (bind _asplayer_base (cast `/Game/Blueprints/Player/Player_Base` BePushed))
  (set `/Game/Blueprints/Player/Player_Base.WhoPushed` WhoPushed _asplayer_base)
  (`KismetSystemLibrary.RetriggerableDelay` 10.0)
  (set `self.WhoPushed` 0))

(event `BeKilled_Multi`
  (params (KillerID :type Integer))
  ;[1 1 1] Add score to the killer
  (bind _outactors (`GameplayStatics.GetAllActorsOfClass` "Player_Base_C"))
  (for _array_element _outactors
    (bind _playerstate (`Pawn.PlayerState` _array_element))
    (`/Engine/EditorBlueprintResources/StandardMacros.IsValid` _playerstate
      (:`Is Valid`
        (if (== (`PlayerState.PlayerId` _playerstate) KillerID)
          (bind _asbp_player_state (cast `/Game/Blueprints/Player/BP_PlayerState` _playerstate))
          (`/Game/Blueprints/Player/BP_PlayerState.Score_Multi` _asbp_player_state (+ (`/Game/Blueprints/Player/BP_PlayerState.PlayerScore` _asbp_player_state) (`self.KillScore`))))))))

(event `Freeze`
  ;[1 1 1] Freeze
  (if (`self.EnableMove`)
    (set `self.EnableMove` false)
    (`/Engine/EditorBlueprintResources/ActorMacros.Switch Has Authority`
      (:`Authority`
        (`self.FreezeAnim_Multi`))
      (:`Remote`
        (`self.FreeAnim_Server`)))
    (`KismetSystemLibrary.Delay` 0.5)
    (set `self.EnableMove` true)))

(event `FreezeAnim_Multi`
  ;[1 1 1] Freeze
  (`self.PlayAnimMontage` "/Game/ArtAssets/scifi/cyborgShock_Anim_Montage.cyborgShock_Anim_Montage" 0.8))

(event `FreeAnim_Server`
  ;[1 1 1] Freeze
  (`self.FreezeAnim_Multi`))

(event `Respawn_Multi`
  (params (PlayerRef :type "/Game/Blueprints/Player/Player_Base Object Reference"))
  (bind _charactermovement (`self.CharacterMovement`))
  ;[1 1 1] Respawn
  (`self.Respawn` PlayerRef)
  (`SceneComponent.K2_SetWorldLocation` (`self.CapsuleComponent`) (`KismetMathLibrary.MakeVector` (.x (`self.SpawnLocation`)) (.y (`self.SpawnLocation`)) (+ (.z (`self.SpawnLocation`)) 100.0)) false true)
  (set `MovementComponent.Velocity` (0.0 0.0 0.0) _charactermovement)
  (`CharacterMovementComponent.DisableMovement` _charactermovement)
  (`SceneComponent.SetVisibility` (`self.Mesh`) false true)
  (`KismetSystemLibrary.Delay` 4.0)
  (`CharacterMovementComponent.SetMovementMode` (`self.CharacterMovement`) "MOVE_Walking" 0)
  (`SceneComponent.SetVisibility` (`self.Mesh`) true true))

(event `Respawn`
  (params (PlayerRef :type "/Game/Blueprints/Player/Player_Base Object Reference"))
  ;[1 1 1] Respawn
  (set `self.EnableMove` false)
  (if (`self.IsLocallyControlled` PlayerRef)
    (bind _asplayer_controller (cast `PlayerController` (`self.GetController`)))
    (bind _returnvalue (`GameplayStatics.GetActorOfClass` "/Game/Blueprints/Level/BP_SpectatingView1.BP_SpectatingView1_C"))
    (`PlayerController.SetViewTargetWithBlend` _asplayer_controller _returnvalue 1.0 "VTBlend_Linear" 0.0 false)
    (`KismetSystemLibrary.Delay` 3.0)
    (bind _asplayer_controller_2 (cast `PlayerController` (`self.GetController`)))
    (`PlayerController.SetViewTargetWithBlend` _asplayer_controller_2 self 1.0 "VTBlend_Linear" 0.0 false)
    (set `self.EnableMove` true)))

(event `GameEnd`
  (bind _asbp_hud (cast `/Game/Blueprints/Player/BP_HUD` (`PlayerController.GetHUD` (`GameplayStatics.GetPlayerController` 0))))
  (`Widget.SetVisibility` (`/Game/Blueprints/Player/BP_HUD.GameUI` _asbp_hud) "Hidden")
  (bind _returnvalue (`|CreateWidget` "/Game/Blueprints/UI/GameOver.GameOver_C"))
  (`UserWidget.AddToViewport` _returnvalue 0)
  (`KismetSystemLibrary.Delay` 1.0)
  (bind _asplayer_controller (cast `PlayerController` (`self.GetController`)))
  (bind _returnvalue_2 (`GameplayStatics.GetActorOfClass` "/Game/Blueprints/Level/BP_SpectatingView.BP_SpectatingView_C"))
  (`PlayerController.SetViewTargetWithBlend` _asplayer_controller _returnvalue_2 1.0 "VTBlend_Linear" 0.0 false))

(event `Time_Multi`
  (params (Time :type "Float (double-precision)"))
  (set `self.Timer` Time))

(fn `OnRep_Dashing`)

(fn `OnRep_MaxScore`)

(fn `OnRep_NewVar_0`)

(fn `OnRep_NewVar_2`)

(fn `OnRep_PlayerName`)

(fn `OnRep_WhoPushed`)

(fn `UserConstructionScript`)