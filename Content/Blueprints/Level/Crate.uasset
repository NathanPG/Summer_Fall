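; Networked crate that knocks back players it hits while moving and can be respawned at its starting spot.
; On overlap, a crate above a speed threshold launches the Player_Base along its velocity, scaled by KnockBackCoefficient, with a short DoOnce cooldown.
; The launch goes through a multicast or server event depending on authority.
; Respawn passes from server to multicast, moving the mesh above its BeginPlay location and clearing linear velocity.
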(event `Respawn_Server`
  (`self.Respawn_Multi`))

(event `Respawn_Multi`
  (bind _staticmesh (`self.StaticMesh`))
  (`SceneComponent.K2_SetWorldLocation` (`self.StaticMesh`) (`KismetMathLibrary.MakeVector` (.x (`self.SpawnLocation`)) (.y (`self.SpawnLocation`)) (+ (.z (`self.SpawnLocation`)) 100.0)) false false)
  (`PrimitiveComponent.SetPhysicsLinearVelocity` _staticmesh (0.0 0.0 0.0) false "None")
  (`PrimitiveComponent.SetAllPhysicsLinearVelocity` _staticmesh (0.0 0.0 0.0) false))

(event `self.ReceiveBeginPlay`
  (set `self.SpawnLocation` (`SceneComponent.K2_GetComponentLocation` (`self.StaticMesh`))))

(event `self.ReceiveActorBeginOverlap`
  (params (OtherActor :type "Actor Object Reference"))
  (bind _returnvalue (`SceneComponent.GetComponentVelocity` (`self.StaticMesh`)))
  (bind _returnvalue_2 (`KismetMathLibrary.VSize` _returnvalue))
  (bind _returnvalue_3 (* (`KismetMathLibrary.Normal` _returnvalue) (* _returnvalue_2 (`self.KnockBackCoefficient`))))
  (`/Engine/EditorBlueprintResources/StandardMacros.DoOnce` false :!label _label
    (:`Completed`
      (`|ExecutionSequence`
        (:`then_0`
          (if (>= _returnvalue_2 50.0)
            (bind _asplayer_base (cast `/Game/Blueprints/Player/Player_Base` OtherActor))
            (`/Engine/EditorBlueprintResources/ActorMacros.Switch Has Authority`
              (:`Authority`
                (`self.Launch_Multi` _asplayer_base _returnvalue_3))
              (:`Remote`
                (`self.Launch_Server` _asplayer_base _returnvalue_3)))))
        (:`then_1`
          (`KismetSystemLibrary.Delay` 0.1)
          (goto _label :!via `Reset`))))))

(event `Launch_Multi`
  (params (Target :type "PlayerCharacter Object Reference (by ref)") (LaunchVelocity :type "Vector Structure"))
  (`Character.LaunchCharacter` Target LaunchVelocity true true))

(event `Launch_Server`
  (params (Target :type "PlayerCharacter Object Reference (by ref)") (LaunchVelocity :type "Vector Structure"))
  (`Character.LaunchCharacter` Target LaunchVelocity true true))

(fn `UserConstructionScript`)