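; Capture point actor that awards score to a player standing alone inside its sphere.
; Sphere overlap events maintain the list and count of players in the point.
; A Delay on Tick throttles scoring to about once per second, with the authority triggering it only when exactly one player is inside.
; Scoring passes the player's score plus PointPerSecond to their PlayerState and subtracts that same total from BonusPool.
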(event `AddScore_Multi`
  (for _array_element (`self.PlayerInPoint`)
    (bind _asbp_player_state (cast `/Game/Blueprints/Player/BP_PlayerState` (`Pawn.PlayerState` _array_element)))
    (bind _returnvalue (+ (`/Game/Blueprints/Player/BP_PlayerState.PlayerScore` _asbp_player_state) (`self.PointPerSecond`)))
    (`/Game/Blueprints/Player/BP_PlayerState.Score_Multi` _asbp_player_state _returnvalue)
    (set `self.BonusPool` (- (`self.BonusPool`) _returnvalue))
    (break)))

(event `self.ReceiveTick`
  (params (DeltaSeconds :type "Float (single-precision)"))
  (`KismetSystemLibrary.Delay` 1.0)
  (if (== (`self.NumberInPoint`) 1)
    (`/Engine/EditorBlueprintResources/ActorMacros.Switch Has Authority`
      (:`Authority`
        (`self.AddScore_Multi`)))))

(event `self.Sphere.OnComponentBeginOverlap`
  (params (OverlappedComponent :type "PrimitiveComponent Object Reference") (OtherActor :type "Actor Object Reference") (OtherComp :type "PrimitiveComponent Object Reference") (OtherBodyIndex :type Integer) (bFromSweep :type Boolean) (SweepResult :type "HitResult Structure (by ref)"))
  (bind _asplayer (cast `/Game/Blueprints/Player/Player` OtherActor))
  (`KismetArrayLibrary.Array_Add` (`self.PlayerInPoint`) _asplayer)
  (`/Engine/EditorBlueprintResources/StandardMacros.IncrementInt` (`self.NumberInPoint`)))

(event `self.Sphere.OnComponentEndOverlap`
  (params (OverlappedComponent :type "PrimitiveComponent Object Reference") (OtherActor :type "Actor Object Reference") (OtherComp :type "PrimitiveComponent Object Reference") (OtherBodyIndex :type Integer))
  (bind _asplayer (cast `/Game/Blueprints/Player/Player` OtherActor))
  (`KismetArrayLibrary.Array_RemoveItem` (`self.PlayerInPoint`) _asplayer)
  (`/Engine/EditorBlueprintResources/StandardMacros.DecrementInt` (`self.NumberInPoint`)))

(fn `UserConstructionScript`)