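; Level pickup actor that grants a buff of its configured Type to a Player overlapping its sphere.
; BeginPlay passes that Type to the BuffWidget on its widget component.
; On pickup it disables collision and hides, then reappears after a short fixed delay, first jumping to a random entry in the Location array when ShouldMove is set.
; An authority check is present but never runs.
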(event `self.Sphere.OnComponentBeginOverlap`
  (params (OverlappedComponent :type "PrimitiveComponent Object Reference") (OtherActor :type "Actor Object Reference") (OtherComp :type "PrimitiveComponent Object Reference") (OtherBodyIndex :type Integer) (bFromSweep :type Boolean) (SweepResult :type "HitResult Structure (by ref)"))
  (bind _location (`self.Location`))
  (bind _asplayer (cast `/Game/Blueprints/Player/Player` OtherActor))
  (`/Game/Blueprints/Player/Player.GetBuff` _asplayer (`self.Type`))
  (`self.SetActorEnableCollision` false)
  (`SceneComponent.SetVisibility` (`self.DefaultSceneRoot`) false true)
  (`KismetSystemLibrary.Delay` 3.0)
  (if (`self.ShouldMove`)
    (`SceneComponent.K2_SetWorldLocation` (`self.DefaultSceneRoot`) (`SceneComponent.K2_GetComponentLocation` (`TargetPoint.SpriteComponent` (`|GetArrayItem` _location (`KismetMathLibrary.RandomIntegerInRange` 0 (- (`KismetArrayLibrary.Array_Length` _location) 1))))) false false))
  (`SceneComponent.SetVisibility` (`self.DefaultSceneRoot`) true true)
  (`self.SetActorEnableCollision` true))

(event `self.ReceiveBeginPlay`
  (bind _asbuff_widget (cast `/Game/Blueprints/UI/BuffWidget` (`WidgetComponent.GetUserWidgetObject` (`self.Widget`))))
  (set `/Game/Blueprints/UI/BuffWidget.Type` (`self.Type`) _asbuff_widget))

(fn `UserConstructionScript`)