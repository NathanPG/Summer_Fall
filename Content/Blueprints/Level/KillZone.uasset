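; KillZone is a level volume that handles anything entering its Box component.
; On the authority, an overlapping Crate is respawned, and an overlapping Player is respawned and then reported killed with its WhoPushed value.
; Any other actor is destroyed without an authority check.
; A disconnected chain of "first" and "second" tag checks remains in the graph and never runs.
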(event `self.Box.OnComponentBeginOverlap`
  (params (OverlappedComponent :type "PrimitiveComponent Object Reference") (OtherActor :type "Actor Object Reference") (OtherComp :type "PrimitiveComponent Object Reference") (OtherBodyIndex :type Integer) (bFromSweep :type Boolean) (SweepResult :type "HitResult Structure (by ref)"))
  (bind _ascrate (cast `/Game/Blueprints/Level/Crate` OtherActor)
    (:`then`
      (`/Engine/EditorBlueprintResources/ActorMacros.Switch Has Authority`
        (:`Authority`
          (`/Game/Blueprints/Level/Crate.Respawn_Multi` _ascrate))))
    (:`CastFailed`
      (bind _asplayer (cast `/Game/Blueprints/Player/Player` OtherActor)
        (:`then`
          (`/Engine/EditorBlueprintResources/ActorMacros.Switch Has Authority`
            (:`Authority`
              (`/Game/Blueprints/Player/Player.Respawn_Multi` _asplayer)
              (`/Game/Blueprints/Player/Player.BeKilled_Multi` _asplayer (`/Game/Blueprints/Player/Player.WhoPushed` _asplayer)))))
        (:`CastFailed`
          (`self.K2_DestroyActor` OtherActor))))))

(fn `UserConstructionScript`)