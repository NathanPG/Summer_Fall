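; Crate is an actor that can be dropped back over its starting point and detects hits on the Player.
; It records its mesh location at BeginPlay, and paired Server and Multi respawn events move the mesh to that XY at a fixed height.
; Hitting a Player only prints a debug message.
; The velocity-scaled knockback, which picks Server or Multi launch events by authority, is disconnected and never runs.
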(event `Respawn_Server`
  (`SceneComponent.K2_SetWorldLocation` (`self.StaticMesh`) (`KismetMathLibrary.MakeVector` (.x (`self.SpawnLocation`)) (.y (`self.SpawnLocation`)) 2000.0) false false))

(event `Respawn_Multi`
  (`SceneComponent.K2_SetWorldLocation` (`self.StaticMesh`) (`KismetMathLibrary.MakeVector` (.x (`self.SpawnLocation`)) (.y (`self.SpawnLocation`)) 2000.0) false false))

(event `self.ReceiveBeginPlay`
  (set `self.SpawnLocation` (`SceneComponent.K2_GetComponentLocation` (`self.StaticMesh`))))

(event `self.ReceiveHit`
  (params (MyComp :type "PrimitiveComponent Object Reference") (Other :type "Actor Object Reference") (OtherComp :type "PrimitiveComponent Object Reference") (bSelfMoved :type Boolean) (HitLocation :type "Vector Structure") (HitNormal :type "Vector Structure") (NormalImpulse :type "Vector Structure") (Hit :type "HitResult Structure (by ref)"))
  (cast `/Game/Blueprints/Player` Other)
  (`KismetSystemLibrary.PrintString` "HIT"))

(event `Launch_Multi`
  (params (Target :type "PlayerCharacter Object Reference (by ref)") (LaunchVelocity :type "Vector Structure"))
  (`Character.LaunchCharacter` Target LaunchVelocity false false))

(event `Launch_Server`
  (params (Target :type "PlayerCharacter Object Reference (by ref)") (LaunchVelocity :type "Vector Structure"))
  (`Character.LaunchCharacter` Target LaunchVelocity false false))

(fn `UserConstructionScript`)