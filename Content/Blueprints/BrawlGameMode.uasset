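; BrawlGameMode is the game mode for a multiplayer brawl, handling player respawns, departures and the host's return to the main menu.
; RespawnPlayer destroys the controller's current pawn, spawns the requested character class at a random PlayerStart and possesses it.
; Controllers from OnSwapPlayerControllers are collected in a list, and a logging-out BrawlPC is passed to GameInfoInstance to destroy its session.
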(event `self.K2_OnSwapPlayerControllers`
  (params (OldPC :type "PlayerController Object Reference") (NewPC :type "PlayerController Object Reference"))
  (`KismetArrayLibrary.Array_Add` (`self.AllPlayerController`) NewPC))

(event `RespawnPlayer`
  (params (PlayerController :type "PlayerController Object Reference") (Character :type "Character Class Reference"))
  (bind _returnvalue (`Controller.K2_GetPawn` PlayerController))
  (bind _spawnpoints (`self.SpawnPoints`))
  (bind _outactors (`GameplayStatics.GetAllActorsOfClass` "/Script/Engine.PlayerStart"))
  (set `self.SpawnPoints` _outactors)
  (`/Engine/EditorBlueprintResources/StandardMacros.IsValid` _returnvalue
    (:`Is Valid`
      (`self.K2_DestroyActor` _returnvalue))
    (:`Is Not Valid`
      _))
  (bind _returnvalue_2 (`|SpawnActorFromClass` Character (`self.GetTransform` (`|GetArrayItem` _spawnpoints (`KismetMathLibrary.RandomIntegerInRange` 0 (- (`KismetArrayLibrary.Array_Length` _spawnpoints) 1)))) "Undefined" "OverrideRootScale" null null))
  (`Controller.Possess` PlayerController _returnvalue_2))

(event `self.K2_OnLogout`
  (params (ExitingController :type "Controller Object Reference"))
  (bind _asbrawl_pc (cast `/Game/Blueprints/BrawlPC` ExitingController))
  (`/Game/Blueprints/GameInfoInstance.DestroySessionCaller` (cast `/Game/Blueprints/GameInfoInstance` (`GameplayStatics.GetGameInstance`) :!pure true) _asbrawl_pc))

(event `HostMainMenu`
  (`self.ReturnToMainMenuHost`)
  (`WidgetBlueprintLibrary.SetInputMode_GameOnly` null))

(fn `UserConstructionScript`
  (`parent.UserConstructionScript`))