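; Replicated multiplayer player character that shoves and dashes into other players, with respawn, score and game-over handling.
; Left click plays a push montage and line-traces to launch players or crates; right click dashes on a Tick-driven cooldown, knocking back players hit.
; Actions branch on authority into Multi or Server events, with client-side crate prediction.
; GameEnd swaps the HUD for a game-over widget and blends to a spectating view.
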(event `self.ReceiveTick`
  (params (DeltaSeconds :type "Float (single-precision)"))
  (`|ExecutionSequence`
    (:`then_0`
      (if (`self.DashCharging`)
        (bind _output_get (set `self.DashCoolDown` (- (`self.DashCoolDown`) DeltaSeconds)))
        (if (<= _output_get 0.0)
          (set `self.DashCharging` false)
          (set `self.DashCoolDown` 3.0))))))

(event `InputAxis|MoveForward` :overrideparent false
  (params (AxisValue :type "Float (single-precision)"))
  (if (`self.Dashing`)
    _
    (elif (`self.EnableMove`)
      (`self.AddMovementInput` (`KismetMathLibrary.GetForwardVector` (`KismetMathLibrary.MakeRotator` 0.0 0.0 (.yaw (`self.GetControlRotation`)))) AxisValue))))

(event `InputAxis|MoveRight` :overrideparent false
  (params (AxisValue :type "Float (single-precision)"))
  (if (`self.Dashing`)
    _
    (elif (`self.EnableMove`)
      (`self.AddMovementInput` (`KismetMathLibrary.GetRightVector` (`KismetMathLibrary.MakeRotator` 0.0 0.0 (.yaw (`self.GetControlRotation`)))) AxisValue))))

(event `InputAxis|Turn` :overrideparent false
  (params (AxisValue :type "Float (single-precision)"))
  (`self.AddControllerYawInput` AxisValue))

(event `self.ReceiveBeginPlay`
  (set `self.SpawnLocation` (`SceneComponent.K2_GetComponentLocation` (`self.CapsuleComponent`)))
  (`self.SetReplicates` true)
  (`self.SetReplicateMovement` true))

(event `Respawn_Server`
  (`SceneComponent.K2_SetWorldLocation` (`self.CapsuleComponent`) (`KismetMathLibrary.MakeVector` (.x (`self.SpawnLocation`)) (.y (`self.SpawnLocation`)) 2000.0) false false))

(event `InputAxis|LookUp` :overrideparent false
  (params (AxisValue :type "Float (single-precision)"))
  (`self.AddControllerPitchInput` AxisValue))

(event `Respawn_Multi`
  (`SceneComponent.K2_SetWorldLocation` (`self.CapsuleComponent`) (`KismetMathLibrary.MakeVector` (.x (`self.SpawnLocation`)) (.y (`self.SpawnLocation`)) 2000.0) false false))

(event `Key|LeftMouseButton`
  (params (Key :type "Key Structure"))
  (bind _returnvalue (`SceneComponent.K2_GetComponentLocation` (`self.CapsuleComponent`)))
  (bind _returnvalue_2 (`KismetMathLibrary.MakeVector` (.x (* (`KismetMathLibrary.Normal` (`self.GetActorForwardVector`)) (`self.PushCrateForce`))) (.y (* (`KismetMathLibrary.Normal` (`self.GetActorForwardVector`)) (`self.PushCrateForce`))) 500.0))
  (:`Pressed`
    (`|ExecutionSequence`
      (:`then_0`
        (`/Engine/EditorBlueprintResources/StandardMacros.DoOnce` false :!label _label
          (:`Completed`
            (`|PlayMontage` (`self.Mesh`) "/Game/ArtAssets/scifi/cyborgpush_Anim_Montage.cyborgpush_Anim_Montage"
              (:`then`
                (bind (_outhit _returnvalue_3) (`KismetSystemLibrary.LineTraceSingle` :`Start` _returnvalue :`End` (+ _returnvalue (* (`KismetMathLibrary.Normal` (`SceneComponent.GetForwardVector` (`self.CapsuleComponent`))) 100.0)) :`TraceChannel` "TraceTypeQuery2" :`DrawDebugType` "ForDuration"))
                (if _returnvalue_3
                  (bind (_bblockinghit _binitialoverlap _time _distance _location _impactpoint _normal _impactnormal _physmat _hitactor) (`GameplayStatics.BreakHitResult` _outhit))
                  (bind _asplayer (cast `/Game/Blueprints/Player` _hitactor)
                    (:`then`
                      (`/Engine/EditorBlueprintResources/ActorMacros.Switch Has Authority`
                        (:`Authority`
                          (bind _returnvalue_4 (`KismetMathLibrary.MakeVector` (.x (* (`KismetMathLibrary.Normal` (- _location (`SceneComponent.K2_GetComponentLocation` (`self.CapsuleComponent`)))) 200.0)) (.y (* (`KismetMathLibrary.Normal` (- _location (`SceneComponent.K2_GetComponentLocation` (`self.CapsuleComponent`)))) 200.0)) 200.0))
                          (`self.Launch_Multi` _asplayer _returnvalue_4))
                        (:`Remote`
                          (`self.Launch_Server` _asplayer _returnvalue_4))))
                    (:`CastFailed`
                      (bind _ascrate (cast `/Game/Blueprints/Crate` _hitactor))
                      (`KismetSystemLibrary.PrintString` "Crate")
                      (`/Engine/EditorBlueprintResources/ActorMacros.Switch Has Authority`
                        (:`Authority`
                          (bind _staticmesh (`/Game/Blueprints/Crate.StaticMesh` _ascrate))
                          (`self.PushCrate_Multi` _staticmesh _returnvalue_2))
                        (:`Remote`
                          (`PrimitiveComponent.AddImpulse` _staticmesh _returnvalue_2 "None" true)
                          (`self.PushCrate_Server` _staticmesh _returnvalue_2)))))))))))
      (:`then_1`
        (`KismetSystemLibrary.Delay` 1.0)
        (goto _label :!via `Reset`)))))

(event `Launch_Server`
  (params (Target :type "PlayerCharacter Object Reference (by ref)") (LaunchVelocity :type "Vector Structure"))
  (`self.LaunchCharacter` Target LaunchVelocity false false))

(event `Launch_Multi`
  (params (Target :type "PlayerCharacter Object Reference (by ref)") (LaunchVelocity :type "Vector Structure"))
  (`self.LaunchCharacter` Target LaunchVelocity false false))

(event `PushCrate_Multi`
  (params (Target :type "PrimitiveComponent Object Reference (by ref)") (LaunchVelocity :type "Vector Structure"))
  (`PrimitiveComponent.AddImpulse` Target LaunchVelocity "None" true))

(event `PushCrate_Server`
  (params (Target :type "PrimitiveComponent Object Reference (by ref)") (LaunchVelocity :type "Vector Structure"))
  (`PrimitiveComponent.AddImpulse` Target LaunchVelocity "None" true))

(event `UpdateMax_Server`
  (params (Max :type "Float (double-precision)") (Name :type Text))
  (set `self.MaxScore` Max))

(event `Key|X`
  (params (Key :type "Key Structure"))
  (bind _playername (`self.PlayerName`))
  (:`Pressed`
    (`KismetSystemLibrary.PrintString` "Add1")
    (bind _output_get (set `self.Score` (+ (`self.Score`) 1.0)))
    (`/Engine/EditorBlueprintResources/StandardMacros.CompareFloat` _output_get (`self.MaxScore`)
      (:`>`
        (`/Engine/EditorBlueprintResources/ActorMacros.Switch Has Authority`
          (:`Authority`
            (`self.UpdateMax_Multi` _playername _output_get))
          (:`Remote`
            (`self.UpdateMax_Server` _output_get _playername)))))))

(event `Key|RightMouseButton`
  (params (Key :type "Key Structure"))
  (bind _returnvalue (`KismetMathLibrary.MakeVector` (.x (* (`KismetMathLibrary.Normal` (`self.GetActorForwardVector`)) (`self.DashVelocity`))) (.y (* (`KismetMathLibrary.Normal` (`self.GetActorForwardVector`)) (`self.DashVelocity`))) 100.0))
  (:`Pressed`
    (if (not (`self.DashCharging`))
      (set `self.DashCharging` true)
      (set `self.Dashing` true)
      (`/Engine/EditorBlueprintResources/ActorMacros.Switch Has Authority`
        (:`Authority`
          (`self.Dash_Multi` self _returnvalue)
          (`KismetSystemLibrary.Delay` 0.3)
          (set `self.Dashing` false))
        (:`Remote`
          (`self.Dash_Server` self _returnvalue)
          (`KismetSystemLibrary.Delay` 0.3)
          (set `self.Dashing` false))))))

(event `Dash_Server`
  (params (Target :type "PlayerCharacter Object Reference (by ref)") (LaunchVelocity :type "Vector Structure"))
  (`self.LaunchCharacter` Target LaunchVelocity false false))

(event `Dash_Multi`
  (params (Target :type "PlayerCharacter Object Reference (by ref)") (LaunchVelocity :type "Vector Structure"))
  (`self.LaunchCharacter` Target LaunchVelocity false false))

(event `Time_Multi`
  (params (Time :type "Float (double-precision)"))
  (set `self.Timer` Time))

(event `UpdateMax_Multi`
  (params (Name :type Text) (Max :type "Float (double-precision)"))
  (set `self.MaxScore` Max))

(event `GameEnd`
  (bind _asbp_hud (cast `/Game/Blueprints/BP_HUD` (`PlayerController.GetHUD` (`GameplayStatics.GetPlayerController` 0))))
  (`Widget.SetVisibility` (`/Game/Blueprints/BP_HUD.GameUI` _asbp_hud) "Hidden")
  (bind _returnvalue (`|CreateWidget` "/Game/Blueprints/GameOver.GameOver_C"))
  (`UserWidget.AddToViewport` _returnvalue 0)
  (`KismetSystemLibrary.Delay` 1.0)
  (bind _asplayer_controller (cast `PlayerController` (`self.GetController`)))
  (bind _returnvalue_2 (`GameplayStatics.GetActorOfClass` "/Game/Blueprints/BP_SpectatingView.BP_SpectatingView_C"))
  (`PlayerController.SetViewTargetWithBlend` _asplayer_controller _returnvalue_2 1.0 "VTBlend_Linear" 0.0 false))

(event `self.ReceiveHit`
  (params (MyComp :type "PrimitiveComponent Object Reference") (Other :type "Actor Object Reference") (OtherComp :type "PrimitiveComponent Object Reference") (bSelfMoved :type Boolean) (HitLocation :type "Vector Structure") (HitNormal :type "Vector Structure") (NormalImpulse :type "Vector Structure") (Hit :type "HitResult Structure (by ref)"))
  (bind _returnvalue (`KismetMathLibrary.MakeVector` (.x (* (`KismetMathLibrary.Normal` (`self.GetActorForwardVector`)) (`self.DashVelocity`))) (.y (* (`KismetMathLibrary.Normal` (`self.GetActorForwardVector`)) (`self.DashVelocity`))) 100.0))
  (if (`self.Dashing`)
    (bind _asplayer (cast `/Game/Blueprints/Player` Other))
    (`KismetSystemLibrary.PrintString` "Dash Hit Player!")
    (`/Engine/EditorBlueprintResources/ActorMacros.Switch Has Authority`
      (:`Authority`
        (`self.DashPush_Multi` _asplayer _returnvalue)
        (set `self.Dashing` false))
      (:`Remote`
        (`self.DashPush_Server` _asplayer _returnvalue)
        (set `self.Dashing` false)))))

(event `DashPush_Multi`
  (params (Target :type "PlayerCharacter Object Reference (by ref)") (LaunchVelocity :type "Vector Structure"))
  (`self.LaunchCharacter` Target LaunchVelocity false false)
  ;[1 1 1] HARD-CODE TIME IF NO HITS
  (`KismetSystemLibrary.Delay` 0.5)
  (set `self.Dashing` false))

(event `DashPush_Server`
  (params (Target :type "PlayerCharacter Object Reference (by ref)") (LaunchVelocity :type "Vector Structure"))
  (`self.LaunchCharacter` Target LaunchVelocity false false)
  ;[1 1 1] HARD-CODE TIME IF NO HITS
  (`KismetSystemLibrary.Delay` 0.5)
  (set `self.Dashing` false))

(fn `OnRep_Dashing`)

(fn `OnRep_MaxScore`)

(fn `OnRep_NewVar_0`)

(fn `OnRep_NewVar_2`)

(fn `UserConstructionScript`)