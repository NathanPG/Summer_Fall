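; BP_LaunchPad is a replicated launch pad that throws Player characters into the air when they enter its sphere trigger.
; The overlap plays a montage on the pad mesh and launches the player along the pad's negative right vector, scaled by LaunchForce, with LaunchHeight as vertical velocity.
; The launch overrides existing velocity and is called directly from the overlap; the server and multicast launch events are not wired into it.
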(event `self.ReceiveBeginPlay`
  (`self.SetReplicates` true)
  (`self.SetReplicateMovement` true))

(event `self.Sphere.OnComponentBeginOverlap`
  (params (OverlappedComponent :type "PrimitiveComponent Object Reference") (OtherActor :type "Actor Object Reference") (OtherComp :type "PrimitiveComponent Object Reference") (OtherBodyIndex :type Integer) (bFromSweep :type Boolean) (SweepResult :type "HitResult Structure (by ref)"))
  (bind _asplayer (cast `/Game/Blueprints/Player` OtherActor))
  (`|PlayMontage` (`self.pad`)
    (:`then`
      (`Character.LaunchCharacter` _asplayer (`KismetMathLibrary.MakeVector` (.x (* (`KismetMathLibrary.Normal` (* (`SceneComponent.GetRightVector` (`self.pad`)) -1.0)) (`self.LaunchForce`))) (.y (* (`KismetMathLibrary.Normal` (* (`SceneComponent.GetRightVector` (`self.pad`)) -1.0)) (`self.LaunchForce`))) (`self.LaunchHeight`)) true true))))

(event `Launch_Multi`
  (params (Target :type "Character Object Reference") (Velocity :type "Vector Structure"))
  (`Character.LaunchCharacter` Target Velocity true true))

(event `Launch_Server`
  (params (Target :type "Character Object Reference") (Velocity :type "Vector Structure"))
  (`Character.LaunchCharacter` Target Velocity true true))

(fn `UserConstructionScript`)