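; MovingPF_BP is a networked moving platform that travels from its starting position to a target Location1.
; On BeginPlay, authority calls the Move_Multi event directly, while remote instances route through Move_Server, which calls the same event.
; Move_Multi caches the actor location as Location0, then plays a timeline that lerps the root component's world location without sweeping.
; Leftover control-point and stop-simulation nodes are never run.
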(event `Move_Server`
  (`self.Move_Multi`))

(event `Move_Multi`
  (set `self.Location 0` (`self.K2_GetActorLocation`))
  (bind (_direction _newtrack_0) (`Timeline|Timeline_0`)
    (:`Update`
      (`SceneComponent.K2_SetWorldLocation` (`self.DefaultSceneRoot`) (`KismetMathLibrary.VLerp` (`self.Location 0`) (`self.Location 1`) _newtrack_0) false false))))

(event `self.ReceiveBeginPlay`
  (`/Engine/EditorBlueprintResources/ActorMacros.Switch Has Authority`
    (:`Authority`
      (`self.Move_Multi`))
    (:`Remote`
      (`self.Move_Server`))))

(fn `UserConstructionScript`)