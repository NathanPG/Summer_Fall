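; Laser turret hazard that spins continuously and freezes any Player its two beams touch.
; Each tick it rotates its root by a fixed step, then line-traces on the Camera channel along each laser component's right vector.
; On a hit, the beam mesh's Y scale shrinks or stretches to the hit distance and a hit Player gets Freeze called.
; Without a hit, the beam resets to a default length.
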(event `self.ReceiveTick`
  (params (DeltaSeconds :type "Float (single-precision)"))
  (bind _laser (`self.Laser`))
  (bind _laser_2 (`self.Laser`))
  (bind _laser0 (`self.Laser0`))
  (bind _laser0_2 (`self.Laser0`))
  (bind _returnvalue (`SceneComponent.K2_GetComponentLocation` _laser0))
  (bind _returnvalue_2 (`SceneComponent.K2_GetComponentLocation` _laser))
  (`SceneComponent.K2_AddLocalRotation` (`self.DefaultSceneRoot`) (struct :`Yaw` 0.5) false false)
  (`|ExecutionSequence`
    (:`then_0`
      (bind (_outhit _returnvalue_3) (`KismetSystemLibrary.LineTraceSingle` _returnvalue_2 (+ _returnvalue_2 (* (`SceneComponent.GetRightVector` _laser) (`self.LaserLength`))) "TraceTypeQuery2"))
      (if _returnvalue_3
        (bind (_bblockinghit _binitialoverlap _time _distance _location _impactpoint _normal _impactnormal _physmat _hitactor _hitcomponent _hitbonename _hititem _faceindex _tracestart) (`GameplayStatics.BreakHitResult` _outhit))
        (`SceneComponent.SetWorldScale3D` _laser_2 (`KismetMathLibrary.MakeVector` 0.04 (/ (`KismetMathLibrary.VSize` (- _tracestart _impactpoint)) 40.0) 0.04))
        (bind _asplayer (cast `/Game/Blueprints/Player` _hitactor))
        (`/Game/Blueprints/Player.Freeze` _asplayer)
        (else
          (`SceneComponent.SetWorldScale3D` _laser_2 (0.04 10.0 0.04)))))
    (:`then_1`
      (bind (_outhit_2 _returnvalue_4) (`KismetSystemLibrary.LineTraceSingle` _returnvalue (+ _returnvalue (* (`SceneComponent.GetRightVector` _laser0) (`self.LaserLength`))) "TraceTypeQuery2"))
      (if _returnvalue_4
        (bind (_bblockinghit_2 _binitialoverlap_2 _time_2 _distance_2 _location_2 _impactpoint_2 _normal_2 _impactnormal_2 _physmat_2 _hitactor_2 _hitcomponent_2 _hitbonename_2 _hititem_2 _faceindex_2 _tracestart_2) (`GameplayStatics.BreakHitResult` _outhit_2))
        (`SceneComponent.SetWorldScale3D` _laser0_2 (`KismetMathLibrary.MakeVector` 0.04 (/ (`KismetMathLibrary.VSize` (- _tracestart_2 _location_2)) 40.0) 0.04))
        (bind _asplayer_2 (cast `/Game/Blueprints/Player` _hitactor_2))
        (`/Game/Blueprints/Player.Freeze` _asplayer_2)
        (else
          (`SceneComponent.SetWorldScale3D` _laser0_2 (0.04 10.0 0.04)))))))

(fn `UserConstructionScript`)