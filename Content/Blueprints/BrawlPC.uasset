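; BrawlPC is the brawl mode player controller that handles character spawning, the game UI and the match-end sequence.
; On local BeginPlay it loads saved player settings, passes them on for BrawlGameMode to respawn the chosen character, then creates the GameUI and hands it to the Player_Base pawn.
; ShowWarning forwards to the pawn.
; GameEnd disables pawn input, swaps to the GameOver widget, blends to a spectating view and enables UI-only input.
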(event `self.ReceiveBeginPlay`
  (if (`self.IsLocalController`)
    (`WidgetLayoutLibrary.RemoveAllWidgets`)
    (`self.LoadGame`)
    (`self.PassCharacterInfoToServer` (`self.PlayerSettings`))
    (bind _returnvalue (`|CreateWidget` "/Game/Blueprints/UI/GameUI.GameUI_C"))
    (bind _output_get (set `self.UI` _returnvalue))
    (`UserWidget.AddToViewport` _output_get 0)
    (bind _asplayer_base (cast `/Game/Blueprints/Player/Player_Base` (`self.K2_GetPawn`)))
    (set `/Game/Blueprints/Player/Player_Base.UI` (`self.UI`) _asplayer_base)
    (`KismetSystemLibrary.PrintString` "Hello")))

(event `PassCharacterInfoToServer`
  (params (PlayerSettingsInfo :type "/Game/Blueprints/PlayerInfo Structure"))
  (set `self.PlayerSettings` PlayerSettingsInfo)
  (bind _asbrawl_game_mode (cast `/Game/Blueprints/BrawlGameMode` (`GameplayStatics.GetGameMode`)))
  (`/Game/Blueprints/BrawlGameMode.RespawnPlayer` _asbrawl_game_mode self (`.MyPlayerCharacter_9_781E5CB143D0AEDF9AC81BBE8372B90E` (break `/Game/Blueprints/PlayerInfo` (`self.PlayerSettings`)))))

(event `ShowWarning`
  (bind _asplayer_base (cast `/Game/Blueprints/Player/Player_Base` (`self.K2_GetPawn`)))
  (`/Game/Blueprints/Player/Player_Base.ShowWarning` _asplayer_base ""))

(event `GameEnd`
  (bind _asplayer_base (cast `/Game/Blueprints/Player/Player_Base` (`self.K2_GetPawn`)))
  (`self.DisableInput` _asplayer_base null)
  (`Widget.SetVisibility` (`self.UI`) "Hidden")
  (bind _returnvalue (`|CreateWidget` "/Game/Blueprints/UI/GameOver.GameOver_C"))
  (`UserWidget.AddToViewport` _returnvalue 0)
  (`KismetSystemLibrary.Delay` 1.0)
  (bind _returnvalue_2 (`GameplayStatics.GetActorOfClass` "/Game/Blueprints/Level/BP_SpectatingView.BP_SpectatingView_C"))
  (`self.SetViewTargetWithBlend` _returnvalue_2 1.0)
  (`WidgetBlueprintLibrary.SetInputMode_UIOnlyEx` null null)
  (set `self.bShowMouseCursor` true))

(fn `LoadGame`
  (bind _returnvalue (`GameplayStatics.LoadGameFromSlot` (`self.PlayerSettingsSave`)))
  (bind _asplayer_save_game (cast `/Game/Blueprints/PlayerSaveGame` _returnvalue))
  (set `self.PlayerSettings` (`/Game/Blueprints/PlayerSaveGame.S_PlayerInfo` _asplayer_save_game)))

(fn `UserConstructionScript`)