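; Falling platform actor that, as wired, sets up vertical InterpToMovement and arms a fall flag when the player steps into its trigger box.
; BeginPlay stores the origin and gives the movement component two relative points with a configurable duration.
; Overlap sets Fall after a short delay, behind a DoOnce that resets later.
; The per-frame drop and return-to-origin logic is disconnected from the empty Tick, so the flag never moves the platform.
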(event `PlatformBack`
  (`SceneComponent.K2_SetWorldLocation` (`self.DefaultSceneRoot`) (`KismetMathLibrary.VLerp` (`SceneComponent.K2_GetComponentLocation` (`self.DefaultSceneRoot`)) (`self.Origin`) 3.0) false false))

(event `self.ReceiveTick`
  (params (DeltaSeconds :type "Float (single-precision)")))

(event `self.Box.OnComponentBeginOverlap`
  (params (OverlappedComponent :type "PrimitiveComponent Object Reference") (OtherActor :type "Actor Object Reference") (OtherComp :type "PrimitiveComponent Object Reference") (OtherBodyIndex :type Integer) (bFromSweep :type Boolean) (SweepResult :type "HitResult Structure (by ref)"))
  (cast `/Game/Blueprints/Player` OtherActor)
  (`/Engine/EditorBlueprintResources/StandardMacros.DoOnce` false :!label _label
    (:`Completed`
      (`KismetSystemLibrary.Delay` 0.2)
      (set `self.Fall` true)
      (`KismetSystemLibrary.Delay` (`self.reset`))
      (goto _label :!via `Reset`))))

(event `self.ReceiveBeginPlay`
  (bind _interptomovement (`self.InterpToMovement`))
  (set `self.Origin` (`SceneComponent.K2_GetComponentLocation` (`self.DefaultSceneRoot`)))
  (set `InterpToMovementComponent.ControlPoints` (`|MakeArray` (make `InterpControlPoint` (0.0 0.0 0.0)) (make `InterpControlPoint` (0.0 0.0 100.0))) _interptomovement)
  (set `InterpToMovementComponent.Duration` (`self.Duration`) _interptomovement))

(fn `UserConstructionScript`)